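; Enemy character with a configurable mesh that starts stationary, chases BP_MainCH and kills it at close range.
; When IsPerseguidor (pursuer) is set, a looping timer sphere-traces ahead and starts a faster chase on a hit.
; CollisionMovement overlap gives pursuers a slower chase and zeroes speed on exit, with AI MoveTo re-issued on success.
; CollisionKill overlap plays a timeline that calls Death on the player when finished, stopped if they leave first.
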(event OnComponentBeginOverlap(CollisionMovement)
  (params (OverlappedComponent :type Primitive%20Component%20Object%20Reference) (OtherActor :type Actor%20Object%20Reference) (OtherComp :type Primitive%20Component%20Object%20Reference) (OtherBodyIndex :type Integer) (bFromSweep :type Boolean) (SweepResult :type Hit%20Result%20Structure%20%28by%20ref%29))
  ;[1 1 1] MoveToPlayer
  (CallFunction|MovetoPlayer (Variables|Default|GetIsPerseguidor) OtherActor :!label _label)
  (AI|AIMoveTo self "0, 0, 0" (Variables|Default|GetObjective) 0.0 false
    (:OnSuccess
      (goto _label))))

(event OnComponentEndOverlap(CollisionMovement)
  (params (OverlappedComponent :type Primitive%20Component%20Object%20Reference) (OtherActor :type Actor%20Object%20Reference) (OtherComp :type Primitive%20Component%20Object%20Reference) (OtherBodyIndex :type Integer))
  ;[1 1 1] MoveToPlayer
  (bind _asbp_main_ch (Utilities|Casting|CastToBP_MainCH OtherActor))
  (Utilities|IsValid _asbp_main_ch
    (:Is%20Valid
      (Variables|Default|SetIsOnCollisionMovement (Variables|Default|GetIsPerseguidor))
      (CallFunction|SetMaxSpeed 0.0))))

(event OnComponentBeginOverlap(CollisionKill)
  (params (OverlappedComponent :type Primitive%20Component%20Object%20Reference) (OtherActor :type Actor%20Object%20Reference) (OtherComp :type Primitive%20Component%20Object%20Reference) (OtherBodyIndex :type Integer) (bFromSweep :type Boolean) (SweepResult :type Hit%20Result%20Structure%20%28by%20ref%29))
  ;[1 1 1] Kill Player
  (bind _asbp_main_ch (Utilities|Casting|CastToBP_MainCH OtherActor))
  (Utilities|IsValid _asbp_main_ch
    (:Is%20Valid
      (bind _output_get (Variables|Default|SetObjective _asbp_main_ch))
      (Timeline|KillTimeLine PlayFromStart
        (:Finished
          (Default|Death _output_get))))))

(event OnComponentEndOverlap(CollisionKill)
  (params (OverlappedComponent :type Primitive%20Component%20Object%20Reference) (OtherActor :type Actor%20Object%20Reference) (OtherComp :type Primitive%20Component%20Object%20Reference) (OtherBodyIndex :type Integer))
  ;[1 1 1] Kill Player
  (bind _asbp_main_ch (Utilities|Casting|CastToBP_MainCH OtherActor))
  (Utilities|IsValid _asbp_main_ch
    (:Is%20Valid
      (Timeline|KillTimeLine Stop
        (:Finished
          (Default|Death (stale OnComponentBeginOverlap(CollisionKill) _output_get)))))))

(event Custom|PulseDetection
  (bind _mesh (Variables|Character|GetMesh))
  (bind _returnvalue (Transformation|GetWorldLocation _mesh))
  ;[1 1 1] PulseDetection
  (bind _output_get (Variables|Default|SetWorldLocationVector (Math|Vector|MakeVector (.x _returnvalue) (.y _returnvalue) (+ (.z _returnvalue) 1.6e+02)) :!label _label))
  (bind _outhit (Collision|SphereTraceByChannel _output_get (+ _output_get (* (Math|Vector|GetForwardVector _mesh) 3e+03)) 1e+02 "TraceTypeQuery1" false 0 "ForDuration" true "(R=1.000000,G=0.000000,B=0.000000,A=1.000000)" "(R=0.000000,G=1.000000,B=0.000000,A=1.000000)" 2.0))
  ;[1 1 1] Moving to Character
  (if (.bBlockingHit (Collision|BreakHitResult _outhit))
    (bind _asbp_main_ch (Utilities|Casting|CastToBP_MainCH (.HitActor (Collision|BreakHitResult _outhit))))
    (bind _output_get_2 (Variables|Default|SetObjective _asbp_main_ch))
    (CallFunction|SetMaxSpeed 2.5e+02)
    (AI|AIMoveTo self "0, 0, 0" _output_get_2 0.0 false
      (:OnSuccess
        (goto _label)))))

(event EventBeginPlay
  (CallFunction|SetMaxSpeed 0.0)
  (if (Variables|Default|GetIsPerseguidor)
    (Utilities|Time|SetTimerbyEvent (delegate Custom|PulseDetection) 5.0 true)))

(event EventTick
  (params (DeltaSeconds :type Float%20%28single-precision%29)))

(fn ConstructionScript
  (Class|SkinnedMeshComponent|SetSkeletalMesh (Variables|Character|GetMesh) (Variables|Default|GetEnemyMesh) true))

(fn SetMaxSpeed
  (params (WalkSpeed :type Float%20%28double-precision%29))
  (Variables|/Script/Engine.CharacterMovementComponent|SetMaxWalkSpeed (Variables|Character|GetCharacterMovement) WalkSpeed))

(fn MovetoPlayer
  (params (IsPerseguidor :type Boolean) (OtherPlayer :type Actor%20Object%20Reference))
  (if IsPerseguidor
    (Variables|Default|SetIsOnCollisionMovement true)
    (bind _asbp_main_ch (Utilities|Casting|CastToBP_MainCH OtherPlayer))
    (Utilities|IsValid _asbp_main_ch
      (:Is%20Valid
        (Variables|Default|SetObjective _asbp_main_ch)
        (CallFunction|SetMaxSpeed 1.5e+02)))))