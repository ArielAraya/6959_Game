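; Reimu NPC actor that talks to the player, takes collected items and can kill them.
; Box overlap branches on the player's item and conversation counters: intro dialogue with view switch, item thanks and removal, or a five-second warning whose timeline ends in Death.
; End overlap increments the conversation counter; InitializeReimu supplies the player reference.
; The eight-item exit phase is a placeholder print, and the construction-positioned Dissapears volume's overlap logic does nothing yet.
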(event OnComponentBeginOverlap(Box)
  (params (OverlappedComponent :type Primitive%20Component%20Object%20Reference) (OtherActor :type Actor%20Object%20Reference) (OtherComp :type Primitive%20Component%20Object%20Reference) (OtherBodyIndex :type Integer) (bFromSweep :type Boolean) (SweepResult :type Hit%20Result%20Structure%20%28by%20ref%29))
  (bind _returnvalue (Game|GetPlayerController 0))
  (bind _returnvalue_2 (Game|GetPlayerController 0))
  (bind _as_bp_main_ch (Variables|Default|GetAs%20BP%20Main%20CH))
  (bind _as_bp_main_ch_2 (Variables|Default|GetAs%20BP%20Main%20CH))
  (bind _as_bp_main_ch_3 (Variables|Default|GetAs%20BP%20Main%20CH))
  (bind _as_bp_main_ch_4 (Variables|Default|GetAs%20BP%20Main%20CH))
  ;[1 1 1] Se verifica al empezar un overlap, que el OTRO actor sea efectivamente el personaje que el jugador controlar.
  (if (== OtherActor (Variables|Default|GetAs%20BP%20Main%20CH))
    (if (and (== (Variables|/Game/MainBranch/Blueprint/PlayerBP/BP_MainCH.BP_MainCH_C|GetContadorObjetos _as_bp_main_ch_2) 0) (== (Variables|/Game/MainBranch/Blueprint/PlayerBP/BP_MainCH.BP_MainCH_C|GetContadorCharlista _as_bp_main_ch_2) 0))
      (bind _returnvalue_3 (UserInterface|CreateWidget "/Game/MainBranch/Blueprint/Widget/WidgetShowBP.WidgetShowBP_C" (Game|GetPlayerController 0)))
      (bind _output_get (Variables|Default|SetWidgetCharlista _returnvalue_3))
      (UserInterface|Viewport|AddtoViewport _output_get 0)
      (Game|Player|SetViewTargetwithBlend _returnvalue self 0.0 "VTBlend_Linear" 0.0 false)
      (bind (_maxwalkspeed _fieldofview) (Default|FovandSpeed _as_bp_main_ch_4))
      (Variables|/Script/Engine.CharacterMovementComponent|SetMaxWalkSpeed (Variables|/Script/Engine.Character|GetCharacterMovement _as_bp_main_ch_4) _maxwalkspeed)
      (Camera|SetFieldOfView (Variables|/Game/MainBranch/Blueprint/PlayerBP/BP_MainCH.BP_MainCH_C|GetCamera (Variables|Default|GetAs%20BP%20Main%20CH)) _fieldofview)
      (Input|DisableInput _as_bp_main_ch_4 _returnvalue)
      (Default|RecibirTexto _returnvalue_3 (Variables|Default|GetTextos_Test))
      (Default|StopRunning _as_bp_main_ch_3)
      (Variables|/Script/Engine.CharacterMovementComponent|SetMaxWalkSpeed (Variables|/Script/Engine.Character|GetCharacterMovement _as_bp_main_ch_3) 1e+02)
      (Camera|SetFieldOfView (Variables|/Game/MainBranch/Blueprint/PlayerBP/BP_MainCH.BP_MainCH_C|GetCamera _as_bp_main_ch_3) 9e+01)
      (elif (and (== (Variables|/Game/MainBranch/Blueprint/PlayerBP/BP_MainCH.BP_MainCH_C|GetContadorObjetos (Variables|Default|GetAs%20BP%20Main%20CH)) 0) (> (Variables|/Game/MainBranch/Blueprint/PlayerBP/BP_MainCH.BP_MainCH_C|GetContadorCharlista (Variables|Default|GetAs%20BP%20Main%20CH)) 0))
        (UserInterface|Viewport|AddtoViewport (Variables|Default|GetWidgetCharlista) 0)
        (Default|RecibirTexto (Variables|Default|GetWidgetCharlista) (Utilities|Array|MakeArray "5 segundos para irte..."))
        (Timeline|DeathTimeLine PlayFromStart
          (:Finished
            (Default|Death (Variables|Default|GetAs%20BP%20Main%20CH))))
        (elif (> (Variables|/Game/MainBranch/Blueprint/PlayerBP/BP_MainCH.BP_MainCH_C|GetContadorObjetos (Variables|Default|GetAs%20BP%20Main%20CH)) 0)
          (bind _item (Default|InformacionArrayEntregar (Variables|Default|GetAs%20BP%20Main%20CH)))
          (if (and (Utilities|Enum|Equal(Enum) _item "NewEnumerator2") (< (Variables|/Game/MainBranch/Blueprint/PlayerBP/BP_MainCH.BP_MainCH_C|GetContadorObjetos (Variables|Default|GetAs%20BP%20Main%20CH)) 8))
            (UserInterface|Viewport|AddtoViewport (Variables|Default|GetWidgetCharlista) 0 :!label _label)
            (Default|RecibirTexto (Variables|Default|GetWidgetCharlista) (Utilities|Array|MakeArray "5 segundos para irte..."))
            (Timeline|Timeline_0 PlayFromStart
              (:Finished
                (Default|Death (Variables|Default|GetAs%20BP%20Main%20CH))))
            (else
              ;[1 1 1] Esto verifica que el jugador tenga 8 o más objetos. de ser el caso, El jugador será capaz de poder empezar a buscar la salida.
              (if (>= (Variables|/Game/MainBranch/Blueprint/PlayerBP/BP_MainCH.BP_MainCH_C|GetContadorObjetos (Variables|Default|GetAs%20BP%20Main%20CH)) 8)
                ;[1 1 1] DEBO HACER QUE REIMU DIGA "PUEDES IRTE" E INICIAR FASE DE CERRADO DE JUEGO
                (Development|PrintString "SEXO")
                (else
                  (bind _returnvalue_4 (UserInterface|CreateWidget "/Game/MainBranch/Blueprint/Widget/WidgetShowBP.WidgetShowBP_C"))
                  (bind _output_get_2 (Variables|Default|SetWidgetCharlista _returnvalue_4))
                  (UserInterface|Viewport|AddtoViewport _output_get_2 0)
                  (Game|Player|SetViewTargetwithBlend _returnvalue_2 self 0.0 "VTBlend_Linear" 0.0 false)
                  (Input|DisableInput (Variables|Default|GetAs%20BP%20Main%20CH) _returnvalue_2)
                  (Default|RecibirTexto (Variables|Default|GetWidgetCharlista) (Utilities|Array|MakeArray (Utilities|Text|ToText(String) (Utilities|String|Append "Arigato gosaimas por tu " (Utilities|String|ToString(Text) (Utilities|Text|ToText(Name) (.SingularDisplayName (Utilities|Struct|BreakFItemStruct (Default|GetItemData (Variables|/Game/MainBranch/Blueprint/PlayerBP/BP_MainCH.BP_MainCH_C|GetBP_InventoryManagerComponent (Variables|Default|GetAs%20BP%20Main%20CH)) _item)))))))))
                  (bind _item_2 (Default|InformacionArrayEntregar _as_bp_main_ch))
                  (Default|InformaciónArrayEliminar _as_bp_main_ch _item_2)
                  (Default|RemoveItem (Variables|/Game/MainBranch/Blueprint/PlayerBP/BP_MainCH.BP_MainCH_C|GetBP_InventoryManagerComponent _as_bp_main_ch) _item_2 1)))))
          (else
            (goto _label)))))))

(event OnComponentEndOverlap(Box)
  (params (OverlappedComponent :type Primitive%20Component%20Object%20Reference) (OtherActor :type Actor%20Object%20Reference) (OtherComp :type Primitive%20Component%20Object%20Reference) (OtherBodyIndex :type Integer))
  (bind _as_bp_main_ch (Variables|Default|GetAs%20BP%20Main%20CH))
  (if (== OtherActor _as_bp_main_ch)
    (Variables|/Game/MainBranch/Blueprint/PlayerBP/BP_MainCH.BP_MainCH_C|SetContadorCharlista _as_bp_main_ch (+ (Variables|/Game/MainBranch/Blueprint/PlayerBP/BP_MainCH.BP_MainCH_C|GetContadorCharlista (Variables|Default|GetAs%20BP%20Main%20CH)) 1))))

(event OnComponentEndOverlap(Dissapears)
  (params (OverlappedComponent :type Primitive%20Component%20Object%20Reference) (OtherActor :type Actor%20Object%20Reference) (OtherComp :type Primitive%20Component%20Object%20Reference) (OtherBodyIndex :type Integer))
  (bind _as_bp_main_ch (Variables|Default|GetAs%20BP%20Main%20CH))
  (bind _contadorobjetos (Variables|/Game/MainBranch/Blueprint/PlayerBP/BP_MainCH.BP_MainCH_C|GetContadorObjetos _as_bp_main_ch))
  (if (== OtherActor _as_bp_main_ch)
    (if (<= (and (== (Math|Integer|%(Integer) _contadorobjetos 2) 0) (> _contadorobjetos 0)) _contadorobjetos)
      _)))

(event EventBeginPlay)

(event Collision|EventActorBeginOverlap
  (params (OtherActor :type Actor%20Object%20Reference)))

(event EventTick
  (params (DeltaSeconds :type Float%20%28single-precision%29)))

(fn ConstructionScript
  (Transformation|SetRelativeLocation (Variables|Default|GetDissapears) (Math|Vector|MakeVector (Variables|Default|GetNew%20Location%20X) (Variables|Default|GetNew%20Location%20Y) (Variables|Default|GetNew%20Location%20Z)) false false)
  (Transformation|SetRelativeScale3D (Variables|Default|GetDissapears) (Math|Vector|MakeVector (Variables|Default|GetNew%20Scale%203D%20X) (Variables|Default|GetNew%20Scale%203D%20Y) (Variables|Default|GetNew%20Scale%203D%20Z))))

(fn InitializeReimu
  (params (As%20BP%20Main%20CH :type BP%20Main%20CH%20Object%20Reference))
  (Variables|Default|SetAs%20BP%20Main%20CH As%20BP%20Main%20CH))