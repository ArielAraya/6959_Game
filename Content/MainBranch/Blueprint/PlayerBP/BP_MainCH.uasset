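; Main player character Blueprint, handling movement, mouse and gamepad look, sprinting and inventory access.
; A timeline blends walk speed and camera FOV for sprinting, while Tick starts idle or walk/run camera shakes based on velocity.
; Toggling the inventory flips IsBeingControlled, which gates movement, look and shake, and pauses the game.
; Helper functions fill, fetch and remove entries in an item-name array and increment an object counter.
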(event Custom|CameraShakeEvent
  (bind _returnvalue (Game|GetPlayerController 0))
  ;[1 1 1] CameraShake
  (if (Variables|Default|GetIsBeingControlled)
    (if (<= (Math|Vector|VectorLength (Transformation|GetVelocity)) 0.0)
      (Game|Feedback|ClientStartCameraShake _returnvalue "/Game/MainBranch/Blueprint/CameraShakeBP/BPCS_Idle.BPCS_Idle_C" 1.0 "CameraLocal" "0,0.000000, 0")
      (else
        (Game|Feedback|ClientStartCameraShake _returnvalue "/Game/MainBranch/Blueprint/CameraShakeBP/BPCS_WalkRun.BPCS_WalkRun_C" 1.0 "CameraLocal" "0, 0, 0")))))

(event Custom|StopRunning
  ;[1 1 1] PlayerRunning - RunningEffect
  (bind _alpha (Timeline|SprintTimeLine SetNewTime)
    (:Update
      (Variables|/Script/Engine.CharacterMovementComponent|SetMaxWalkSpeed (Variables|Character|GetCharacterMovement) (Math|Float|Lerp (Variables|Default|GetWalkSpeed) (Variables|Default|GetRunSpeed) _alpha))
      (Camera|SetFieldOfView (Variables|Default|GetCamera) (Math|Float|Lerp (Variables|Default|GetMinFieldOfView) (Variables|Default|GetMaxFieldOfView) _alpha)))))

(event EventBeginPlay
  (CallFunction|InicializarVariables)
  (Default|RemoveItem (Variables|Default|GetBP_InventoryManagerComponent) "NewEnumerator0" 1))

(event Collision|EventActorBeginOverlap
  (params (OtherActor :type Actor%20Object%20Reference)))

(event EventTick
  (params (DeltaSeconds :type Float%20%28single-precision%29))
  (CallFunction|CameraShakeEvent))

(event Input|ActionEvents|InputActionRun
  (params (Key :type Key%20Structure :default "None"))
  ;[1 1 1] PlayerRunning - RunningEffect
  (:Pressed
    (if (Variables|Default|GetIsBeingControlled)
      (if (not (<= (Math|Vector|VectorLength (Transformation|GetVelocity)) 0.0))
        (Variables|Default|SetisRunning true)
        (if (Variables|Default|GetisRunning) :!label _label
          (bind _alpha (Timeline|SprintTimeLine Play)
            (:Update
              (Variables|/Script/Engine.CharacterMovementComponent|SetMaxWalkSpeed (Variables|Character|GetCharacterMovement) (Math|Float|Lerp (Variables|Default|GetWalkSpeed) (Variables|Default|GetRunSpeed) _alpha))
              (Camera|SetFieldOfView (Variables|Default|GetCamera) (Math|Float|Lerp (Variables|Default|GetMinFieldOfView) (Variables|Default|GetMaxFieldOfView) _alpha))))
          (else
            (Timeline|SprintTimeLine Reverse))))))
  (:Released
    (if (Variables|Default|GetIsBeingControlled)
      _
      (else
        _))
    (Variables|Default|SetisRunning false)
    (goto _label)))

(event Input|ActionEvents|InputActionOpenInventory
  (params (Key :type Key%20Structure :default "None"))
  ;[1 1 1] Toggle if the inventory is open or not!
  (:Pressed
    (Default|ToggleInventoryOpen (Variables|Default|GetInventoryManager))
    ;[1 1 1] Gain and Loose control over the character. In  here to save a cast!
    (bind _output_get (Variables|Default|SetIsBeingControlled (not (Variables|Default|GetIsBeingControlled))))
    (if _output_get
      (Game|SetGamePaused false)
      (else
        (Game|SetGamePaused true)))))

(event Input|AxisEvents|InputAxisTurn
  (params (AxisValue :type Float%20%28single-precision%29))
  ;[0.2789 0.5951 1] Mouse camera control
  (if (Variables|Default|GetIsBeingControlled)
    (Pawn|Input|AddControllerYawInput (* (* AxisValue (Utilities|Time|GetWorldDeltaSeconds)) (Variables|Default|GetMouseSensetivity)))))

(event Input|AxisEvents|InputAxisLookUp
  (params (AxisValue :type Float%20%28single-precision%29))
  ;[0.2789 0.5951 1] Mouse camera control
  (if (Variables|Default|GetIsBeingControlled)
    (Pawn|Input|AddControllerPitchInput (* (* (Utilities|Time|GetWorldDeltaSeconds) AxisValue) (Variables|Default|GetMouseSensetivity)))))

(event Input|AxisEvents|InputAxisMoveForward
  (params (AxisValue :type Float%20%28single-precision%29))
  ;[1 1 1] PlayerMovement
  (if (Variables|Default|GetIsBeingControlled)
    (Pawn|Input|AddMovementInput (Transformation|GetActorForwardVector) AxisValue false)))

(event Input|AxisEvents|InputAxisMoveRight
  (params (AxisValue :type Float%20%28single-precision%29))
  ;[1 1 1] PlayerMovement
  (if (Variables|Default|GetIsBeingControlled)
    (Pawn|Input|AddMovementInput (Transformation|GetActorRightVector) AxisValue false)))

(event Input|AxisEvents|InputAxisTurnRate
  (params (AxisValue :type Float%20%28single-precision%29))
  ;[0.1477 0.5585 1] Joystick camera control
  (if (Variables|Default|GetIsBeingControlled)
    (Pawn|Input|AddControllerYawInput (* AxisValue (Variables|Default|GetBaseTurnRate) (Utilities|Time|GetWorldDeltaSeconds)))))

(event Input|AxisEvents|InputAxisLookUpRate
  (params (AxisValue :type Float%20%28single-precision%29))
  ;[0.1477 0.5585 1] Joystick camera control
  (if (Variables|Default|GetIsBeingControlled)
    (Pawn|Input|AddControllerPitchInput (* AxisValue (Variables|Default|GetBaseLookUpRate) (Utilities|Time|GetWorldDeltaSeconds)))))

(fn ConstructionScript
  (Utilities|FlowControl|Sequence
    (:then_0
      (Variables|/Script/Engine.CharacterMovementComponent|SetMaxWalkSpeed (Variables|Character|GetCharacterMovement) (Variables|Default|GetWalkSpeed)))))

(fn Death)

(fn InicializarVariables
  (Variables|Default|SetContadorObjetos 0)
  (Variables|Default|SetContadorCharlista 0)
  (bind _inventorymanagercomponent (CallFunction|GetInventoryManager self))
  (Variables|Default|SetInventoryManager _inventorymanagercomponent))

(fn InformaciónArrayObtener
  (params (NewItem :type EItems%20Enum :default "NewEnumerator0"))
  (bind (_array_element _array_index) (Utilities|Array|ForEachLoopwithBreak (Variables|Default|GetArrayItemName) :!label _label)
    (:LoopBody
      (if (Utilities|Enum|Equal(Enum) _array_element "NewEnumerator2")
        (Utilities|Array|SetArrayElem (Variables|Default|GetArrayItemName) _array_index NewItem)
        (goto _label Break)))
    (:Completed
      (return))))

(fn InformacionArrayEntregar
  (bind (_array_element _array_index) (Utilities|Array|ForEachLoopwithBreak (Variables|Default|GetArrayItemName) :!label _label)
    (:LoopBody
      (if (not (Utilities|Enum|Equal(Enum) _array_element "NewEnumerator2"))
        (LocalVariables|SetItemAEntregar (Utilities|Array|Get(acopy) (Variables|Default|GetArrayItemName) _array_index))
        (goto _label Break)))
    (:Completed
      (return (LocalVariables|GetItemAEntregar)))))

(fn AumentarContador
  (Variables|Default|SetContadorObjetos (+ (Variables|Default|GetContadorObjetos) 1))
  (return))

(fn InformaciónArrayEliminar
  (params (ItemEliminar :type EItems%20Enum :default "NewEnumerator0"))
  (bind (_array_element _array_index) (Utilities|Array|ForEachLoopwithBreak (Variables|Default|GetArrayItemName) :!label _label)
    (:LoopBody
      (if (Utilities|Enum|Equal(Enum) _array_element ItemEliminar)
        (Utilities|Array|RemoveIndex (Variables|Default|GetArrayItemName) _array_index)
        (goto _label Break)))
    (:Completed
      (return))))

(fn FovandSpeed
  (return (Variables|/Script/Engine.CharacterMovementComponent|GetMaxWalkSpeed (Variables|Character|GetCharacterMovement)) (Variables|/Script/Engine.CameraComponent|GetFieldOfView (Variables|Default|GetCamera))))